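; FishBaseBP is a base fish actor that scores points when the player grabs and then releases it.
; On BeginPlay it finds the GameManagerBP and binds to its FishGrabComponent's grabbed and dropped events.
; Grabbing does nothing; dropping adds PointValue through the manager, spawns a scaled-down FishExplosionBP at the grab component, optionally grants more air via GiveAir, then destroys the fish.
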(event Custom|OnGrabbed_Event)

(event Custom|OnDropped_Event
  (bind _gamemanager (Variables|Default|GetGameManager))
  (Default|AddPoints _gamemanager (Variables|Default|GetpointValue))
  (Game|SpawnActorfromClass "/Game/Fishies/FishExplosionBP.FishExplosionBP_C" (Math|Transform|MakeTransform (Transformation|GetWorldLocation (Variables|Default|GetFishGrabComponent)) "0, 0, 0" (Math|Conversions|ToVector(Float) (Math|Float|MakeLiteralFloat 0.3))) "Undefined" 0 0)
  (if (Variables|Default|GetgiveAir)
    (Default|MoreAir _gamemanager))
  (Actor|DestroyActor))

(event EventBeginPlay
  (bind _fishgrabcomponent (Variables|Default|GetFishGrabComponent))
  (bind _returnvalue (Actor|GetActorOfClass "/Game/GameManagerBP.GameManagerBP_C"))
  (Variables|Default|SetGameManager _returnvalue)
  (if (Utilities|IsValid _fishgrabcomponent)
    (EventDispatchers|AssignOnGrabbed _fishgrabcomponent (delegate Custom|OnGrabbed_Event))
    (EventDispatchers|AssignOnDropped _fishgrabcomponent (delegate Custom|OnDropped_Event))))

(fn ConstructionScript)