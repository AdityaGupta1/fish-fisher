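; GameManagerBP is a game manager that tracks the player's score and a draining oxygen supply.
; Oxygen resets on BeginPlay and falls in real time on Tick, clamped at zero.
; When oxygen runs low, Tick writes a scaled value to the Progress parameter of the M_VR_params material parameter collection.
; AddPoints raises Score, and MoreAir tops up oxygen by a fixed amount.
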(event EventBeginPlay
  (Variables|Default|SetOxygen 1e+02))

(event EventTick
  (params (DeltaSeconds :type Float%20%28single-precision%29))
  (bind _output_get (Variables|Default|SetOxygen (- (Variables|Default|GetOxygen) DeltaSeconds)))
  (if (< _output_get 3e+01)
    (Rendering|Material|SetScalarParameterValue "/Game/Assets/Materials/M_VR_params.M_VR_params" "Progress" (/ (Variables|Default|GetOxygen) 15.0) :!class /Script/Engine.KismetMaterialLibrary)
    (if (< (Variables|Default|GetOxygen) 0.0)
      (Variables|Default|SetOxygen 0.0))))

(fn ConstructionScript)

(fn AddPoints
  (params (Points%20To%20Add :type Integer))
  (Variables|Default|SetScore (+ Points%20To%20Add (Variables|Default|GetScore))))

(fn MoreAir
  (Variables|Default|SetOxygen (+ 2e+01 (Variables|Default|GetOxygen))))